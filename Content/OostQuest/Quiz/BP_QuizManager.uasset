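; Quiz manager actor that runs per-location quizzes and awards a collectable mesh upon completion.
; StartQuiz builds the question widget and answer buttons from the QuizQuestions map, and each correct answer advances to the next question.
; After the last one, an unowned collectable appears on the player's CollectableMesh, rotated by a looping timer, with a congratulation widget.
; A shrink timer later clears it, marks it acquired and resets the selected point of interest.
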(event Custom|StartShrinkingCollectable
  ;[1 1 1] Calls the timer and the function for shrinking collectables on the screen.
  (bind _returnvalue (Utilities|Time|SetTimerbyEvent (delegate Custom|ShrinkCollectable) (Variables|Collectables|GetShrinkInterval) true)))

(event Custom|ShrinkCollectable
  ;[1 1 1] Calls the timer and the function for shrinking collectables on the screen.
  (CallFunction|ShrinkCollectableFunction (stale Custom|StartShrinkingCollectable _returnvalue)))

(event Custom|StartRotatingCollectable
  ;[1 1 1] Rotates the collectable on the screen.
  (Utilities|Time|SetTimerbyEvent (delegate Custom|RotateCollectableEvent) (Variables|Collectables|GetRotationInterval) true))

(event Custom|RotateCollectableEvent
  ;[1 1 1] Rotates the collectable on the screen.
  (Transformation|AddWorldRotation (Variables|/Game/TopDown/Blueprints/BP_TopDownCharacter.BP_TopDownCharacter_C|GetCollectableMesh (Variables|References|GetPlayerRef)) (Math|Rotator|MakeRotator 0.0 0.0 (Variables|Collectables|GetRotationSpeed)) false false))

(event EventBeginPlay
  ;[1 1 1] Sets the player reference.
  (bind _asbp_top_down_character (Utilities|Casting|CastToBP_TopDownCharacter (Game|Player|GetPlayerPawn 0)))
  (Variables|References|SetPlayerRef _asbp_top_down_character))

(event Collision|EventActorBeginOverlap
  (params (OtherActor :type Actor%20Object%20Reference)))

(event EventTick
  (params (DeltaSeconds :type Float%20%28single-precision%29)))

(fn ConstructionScript)

(fn StartQuiz
  (params (LocationName :type E_LocationEnum%20Enum :default "NewEnumerator0") (CurrentQuestion :type Integer))
  ;[1 1 1] Puts the first question of a quiz on screen. The current quiz and question indexes are saved for later use.
  (Utilities|Platform|CollectGarbage)
  (Variables|Quiz|SetCurrentQuiz LocationName)
  (Variables|Quiz|SetCurrentQuestion CurrentQuestion)
  (bind _returnvalue (UserInterface|CreateWidget "/Game/OostQuest/Quiz/Widgets/WBP_QuizMenu.WBP_QuizMenu_C" 0 (.question (Utilities|Array|Get(acopy) (.quizquestion (.Value (Utilities|Map|Find (Variables|Quiz|GetQuizQuestions) LocationName))) (Variables|Quiz|GetCurrentQuestion)))))
  (bind _output_get (Variables|References|SetQuizMenuRef _returnvalue))
  (UserInterface|Viewport|AddtoViewport _output_get 0)
  (for _array_element (.answers (Utilities|Array|Get(acopy) (.quizquestion (.Value (Utilities|Map|Find (Variables|Quiz|GetQuizQuestions) LocationName))) (Variables|Quiz|GetCurrentQuestion)))
    (Default|AddButton (Variables|References|GetQuizMenuRef) (.answer _array_element) (.correct? _array_element)))
  (return))

(fn QuestionAnsweredCorrectly
  (bind _currentquiz (Variables|Quiz|GetCurrentQuiz))
  (bind _quizquestions (Variables|Quiz|GetQuizQuestions))
  (bind _value (Utilities|Map|Find _quizquestions _currentquiz))
  ;[1 1 1] Once a quiz question has been answered correctly, the quiz goes to the next one. If there is no next one, the collectable is given to the player (if he doesn't already own it).
  (LocalVariables|SetCollectable (.collectable _value))
  (bind _result (Math|Integer|IncrementInt (Variables|Quiz|GetCurrentQuestion))
    (:%20%20
      (Widget|RemovefromParent (Variables|References|GetQuizMenuRef))
      (Utilities|Platform|CollectGarbage)
      (Variables|References|SetQuizMenuRef 0)
      (if (Utilities|Array|IsValidIndex (.quizquestion _value) _result)
        (CallFunction|StartQuiz (Variables|Quiz|GetCurrentQuiz) (Variables|Quiz|GetCurrentQuestion))
        (return)
        (elif (not (.collectableacquired? _value))
          (Components|StaticMesh|SetStaticMesh (Variables|/Game/TopDown/Blueprints/BP_TopDownCharacter.BP_TopDownCharacter_C|GetCollectableMesh (Variables|References|GetPlayerRef)) (LocalVariables|GetCollectable))
          ;;[0 0 1] Added widget for the text below a collectable.
          (bind _returnvalue (UserInterface|CreateWidget "/Game/OostQuest/Quiz/Widgets/WBP_CollectableAcquired.WBP_CollectableAcquired_C" 0 (Utilities|Text|ToText(String) (Utilities|String|Append "Gefeliciteerd! Je hebt " (Utilities|GetDisplayName (LocalVariables|GetCollectable)) " gevonden."))))
          (bind _output_get (Variables|References|SetCollectableAcquiredRef _returnvalue))
          (UserInterface|Viewport|AddtoViewport _output_get 0)
          (CallFunction|StartRotatingCollectable)
          (Variables|Collectables|SetCollectableOnScreen true)
          (return)
          (else
            (Default|ResetInteractableDoOnce (Variables|References|GetSelectedPointOfInterestRef))
            (return)))))))

(fn ShrinkCollectableFunction
  (params (TimerHandle :type Timer%20Handle%20Structure))
  (bind _quizquestions (Variables|Quiz|GetQuizQuestions))
  (bind _currentquiz (Variables|Quiz|GetCurrentQuiz))
  (bind _playerref (Variables|References|GetPlayerRef))
  (bind _playerref_2 (Variables|References|GetPlayerRef))
  (bind _value (Utilities|Map|Find _quizquestions _currentquiz))
  (bind _collectablemesh (Variables|/Game/TopDown/Blueprints/BP_TopDownCharacter.BP_TopDownCharacter_C|GetCollectableMesh _playerref_2))
  (bind _collectablemesh_2 (Variables|/Game/TopDown/Blueprints/BP_TopDownCharacter.BP_TopDownCharacter_C|GetCollectableMesh _playerref))
  ;[1 1 1] Collectable shrinks to 0, 0, 0 scale and disappears off screen. The timer for this is reset after and the scale for the collectable slot as well.
  (Widget|RemovefromParent (Variables|References|GetCollectableAcquiredRef))
  (Utilities|Platform|CollectGarbage)
  (if (>= (.x (Variables|/Script/Engine.SceneComponent|GetRelativeScale3D (Variables|/Game/TopDown/Blueprints/BP_TopDownCharacter.BP_TopDownCharacter_C|GetCollectableMesh (Variables|References|GetPlayerRef)))) 0.0)
    (Transformation|SetRelativeScale3D _collectablemesh_2 (- (Variables|/Script/Engine.SceneComponent|GetRelativeScale3D _collectablemesh_2) (Variables|Collectables|GetShrinkSpeed)))
    (else
      (Utilities|Map|Add _quizquestions _currentquiz (Utilities|Struct|MakeS_QuizQuestionSet (.quizquestion _value) (.collectable _value) true))
      (Components|StaticMesh|SetStaticMesh _collectablemesh 0)
      (Variables|Collectables|SetCollectableOnScreen false)
      (Utilities|Time|ClearandInvalidateTimerbyHandle TimerHandle)
      (Transformation|SetRelativeScale3D _collectablemesh "1.000000,1.000000,1.000000")
      (Default|ResetInteractableDoOnce (Variables|References|GetSelectedPointOfInterestRef)))))

(fn RemoveWidgets
  (params (ToRemove :type Array%20of%20Widget%20Object%20References))
  ;[0 0 1] Removes multiple widgets from the screen.
  (for _array_element ToRemove
    (Widget|RemovefromParent _array_element))
  (Utilities|Platform|CollectGarbage)
  (return))