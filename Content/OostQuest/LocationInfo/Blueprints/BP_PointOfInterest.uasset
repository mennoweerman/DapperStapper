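; BP_PointOfInterest is a clickable location actor that opens an information widget for its named place.
; Its construction script looks up LocationName in LocationMap and sets the matching building mesh.
; Clicking the mesh passes that entry's info array and name to a new WBP_PointInformation in the viewport, or prints an error for unknown names.
; A DoOnce limits this to one click, with no reset wired here.
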(event OnClicked(StaticMesh)
  (params (TouchedComponent :type Primitive%20Component%20Object%20Reference) (ButtonPressed :type Key%20Structure :default "None"))
  (bind _locationmap (Variables|LocationSettings|GetLocationMap))
  (bind _locationname (Variables|LocationSettings|GetLocationName))
  (bind (_value _returnvalue) (Utilities|Map|Find _locationmap _locationname))
  ;[1 1 1] When the mesh is clicked, check if the location name exists. When true, create the info widget
  ;;[1 1 0] Reset after quiz
  (Utilities|FlowControl|DoOnce false
    (:Completed
      (if _returnvalue
        (bind _returnvalue_2 (UserInterface|CreateWidget "/Game/OostQuest/LocationInfo/Widgets/WBP_PointInformation.WBP_PointInformation_C" 0 (.locationinfoarray _value) _locationname))
        (UserInterface|Viewport|AddtoViewport _returnvalue_2 0)
        (else
          (Development|PrintString "ERROR: Location name does not exist in BP_PointOfInterest" true true "(R=1.000000,G=0.000000,B=0.000000,A=1.000000)" 1e+01))))))

(fn ConstructionScript
  (bind _locationname (Variables|LocationSettings|GetLocationName))
  (bind _locationmap (Variables|LocationSettings|GetLocationMap))
  (bind (_value _returnvalue) (Utilities|Map|Find _locationmap _locationname))
  ;[1 1 1] On construct, changes the mesh of the point of interest
  (if _returnvalue
    (Components|StaticMesh|SetStaticMesh (Variables|Default|GetStaticMesh) (.buildingmesh _value))))