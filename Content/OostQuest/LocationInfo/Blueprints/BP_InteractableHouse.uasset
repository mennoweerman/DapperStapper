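; Clickable house actor that represents a named location and shows information about it.
; On begin play it looks up LocationName in LocationMap and sets its static mesh to that entry's building model.
; Clicking the mesh looks up the location again and opens a WBP_PointInformation widget filled with that entry's info array, or prints an error if the name is missing.
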(event OnClicked(StaticMesh)
  (params (TouchedComponent :type Primitive%20Component%20Object%20Reference) (ButtonPressed :type Key%20Structure :default "None"))
  ;[0 0 1] When the mesh is clicked, cast to the house blueprint and check if the location name exists. When true, create the info widget
  (bind _asbp_interactable_house (Utilities|Casting|CastToBP_InteractableHouse (Components|GetOwner TouchedComponent)))
  (if (.ReturnValue (Utilities|Map|Find (Variables|LocationSettings|GetLocationMap) (Variables|BP_InteractableHouse_C|GetLocationName _asbp_interactable_house)))
    (bind _returnvalue (UserInterface|CreateWidget "/Game/OostQuest/LocationInfo/Widgets/WBP_PointInformation.WBP_PointInformation_C" 0 (.locationinfoarray (.Value (Utilities|Map|Find (Variables|LocationSettings|GetLocationMap) (Variables|BP_InteractableHouse_C|GetLocationName _asbp_interactable_house))))))
    (UserInterface|Viewport|AddtoViewport _returnvalue 0)
    (else
      (Development|PrintString "Location name does not exist"))))

(event EventBeginPlay
  (bind _locationname (Variables|LocationSettings|GetLocationName))
  (bind _locationmap (Variables|LocationSettings|GetLocationMap))
  (bind (_value _returnvalue) (Utilities|Map|Find _locationmap _locationname))
  ;[0 0 1] On begin play, sets the model of the correct building
  (if _returnvalue
    (Components|StaticMesh|SetStaticMesh (Variables|Default|GetStaticMesh) (.buildingmodel _value))))

(fn ConstructionScript)