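; Quiz manager that runs per-location question sets and awards a collectable when a set is completed.
; StartQuiz builds the quiz widget and animates the player's mascot mesh; correct answers advance until the collectable appears with Dutch found or already-owned text.
; Looping timers, rather than Tick, spin the player's item mesh and, once triggered, shrink it away.
; When shrinking ends, it records the collection entry, saves, and has the map spline give a hint.
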(event Custom|StartShrinkingCollectable
  ;[1 1 1] Calls the timer and the function for shrinking collectables on the screen.
  (bind _returnvalue (Utilities|Time|SetTimerbyEvent (delegate Custom|ShrinkCollectable) (Variables|Collectables|GetShrinkInterval) true)))

(event Custom|ShrinkCollectable
  ;[1 1 1] Calls the timer and the function for shrinking collectables on the screen.
  (CallFunction|ShrinkCollectableFunction (stale Custom|StartShrinkingCollectable _returnvalue)))

(event Custom|StartRotatingCollectable
  ;[1 1 1] Rotates the collectable on the screen.
  (Utilities|Time|SetTimerbyEvent (delegate Custom|RotateCollectableEvent) (Variables|Collectables|GetRotationInterval) true))

(event Custom|RotateCollectableEvent
  ;[1 1 1] Rotates the collectable on the screen.
  (Transformation|AddLocalRotation (Variables|/Game/TopDownBP/Blueprints/TopDownCharacter.TopDownCharacter_C|GetItemMesh (Variables|References|GetPlayerRef)) (Math|Rotator|MakeRotator 0.0 0.0 (Variables|Collectables|GetRotationSpeed)) false false))

(event EventBeginPlay
  ;[1 1 1] Sets the player reference.
  (CallFunction|StartRotatingCollectable)
  (bind _astop_down_character (Utilities|Casting|CastToTopDownCharacter (Game|Player|GetPlayerPawn 0)))
  (Variables|References|SetPlayerRef _astop_down_character)
  ;[1 1 1] Sets Save Manager Ref and reference to all points of interest
  (bind _returnvalue (Actor|GetActorOfClass "/Game/DapperStapper/Save/BP_SaveManager.BP_SaveManager_C"))
  (Variables|References|SetSaveManagerRef _returnvalue)
  (bind _outactors (Actor|GetAllActorsOfClass "/Game/DapperStapper/LocationInfo/Blueprints/BP_PointOfInterest.BP_PointOfInterest_C"))
  (Variables|References|SetPointsOfInterestRef _outactors)
  (bind _returnvalue_2 (Actor|GetActorOfClass "/Game/DapperStapper/HintsAlongRoute/Blueprints/BP_MapSpline.BP_MapSpline_C"))
  (Variables|References|SetMapSplineRef _returnvalue_2))

(fn ConstructionScript)

(fn ShrinkCollectableFunction
  (params (TimerHandle :type Timer%20Handle%20Structure))
  (bind _playerref (Variables|References|GetPlayerRef))
  (bind _playerref_2 (Variables|References|GetPlayerRef))
  (bind _itemmesh (Variables|/Game/TopDownBP/Blueprints/TopDownCharacter.TopDownCharacter_C|GetItemMesh _playerref_2))
  (bind _itemmesh_2 (Variables|/Game/TopDownBP/Blueprints/TopDownCharacter.TopDownCharacter_C|GetItemMesh _playerref))
  ;[1 1 1] Collectable shrinks to 0, 0, 0 scale and disappears off screen. The timer for this is reset after and the scale for the collectable slot as well.
  (Widget|RemovefromParent (Variables|References|GetCollectableAcquiredRef))
  (Utilities|Platform|CollectGarbage)
  (if (>= (.x (Variables|/Script/Engine.SceneComponent|GetRelativeScale3D (Variables|/Game/TopDownBP/Blueprints/TopDownCharacter.TopDownCharacter_C|GetItemMesh (Variables|References|GetPlayerRef)))) 0.0)
    (Transformation|SetRelativeScale3D _itemmesh_2 (- (Variables|/Script/Engine.SceneComponent|GetRelativeScale3D _itemmesh_2) (Variables|Collectables|GetShrinkSpeed)))
    (return)
    (else
      (Utilities|Map|Add (Variables|/Game/DapperStapper/Save/BP_SaveGame.BP_SaveGame_C|GetCollectionMap (Variables|/Game/DapperStapper/Save/BP_SaveManager.BP_SaveManager_C|GetSaveGameRef (Variables|References|GetSaveManagerRef))) (Variables|Quiz|GetCurrentQuiz) true)
      (Components|StaticMesh|SetStaticMesh _itemmesh 0)
      (Variables|Collectables|SetCollectableOnScreen false)
      (Utilities|Time|ClearandInvalidateTimerbyHandle TimerHandle)
      (Transformation|SetRelativeScale3D _itemmesh "1.000000,1.000000,1.000000")
      (Default|SaveGame (Variables|References|GetSaveManagerRef))
      (Default|GiveHinttoPlayer (Variables|References|GetMapSplineRef))
      (return))))

(fn QuestionAnsweredCorrectly
  (bind _currentquiz (Variables|Quiz|GetCurrentQuiz))
  (bind _quizquestions (Variables|Quiz|GetQuizQuestions))
  (bind _value (Utilities|Map|Find _quizquestions _currentquiz))
  ;[1 1 1] Once a quiz question has been answered correctly, the quiz goes to the next one. If there is no next one, the collectable is given to the player (if he doesn't already own it).
  (LocalVariables|SetCollectable (.collectable _value))
  (bind _result (Math|Integer|IncrementInt (Variables|Quiz|GetCurrentQuestion))
    (:%20%20
      (Widget|RemovefromParent (Variables|References|GetQuizMenuRef))
      (Utilities|Platform|CollectGarbage)
      (Variables|References|SetQuizMenuRef 0)
      (if (Utilities|Array|IsValidIndex (.quizquestion _value) _result)
        (CallFunction|StartQuiz (Variables|Quiz|GetCurrentQuiz) (Variables|Quiz|GetCurrentQuestion))
        (return)
        (else
          (CallFunction|PutCollectableonScreen (LocalVariables|GetCollectable) (.collectablemeshscale _value) (Variables|Quiz|GetCurrentQuiz))
          (return))))))

(fn StartQuiz
  (params (LocationName :type E_LocationEnum%20Enum :default "NewEnumerator0") (CurrentQuestion :type Integer))
  (bind _playerref (Variables|References|GetPlayerRef))
  (bind _quizinfomesh (Variables|/Game/TopDownBP/Blueprints/TopDownCharacter.TopDownCharacter_C|GetQuizInfoMesh _playerref))
  ;[1 1 1] Puts the first question of a quiz on screen. The current quiz and question indexes are saved for later use.
  (Utilities|Platform|CollectGarbage)
  (Variables|Quiz|SetCurrentQuiz LocationName)
  (Variables|Quiz|SetCurrentQuestion CurrentQuestion)
  (bind _returnvalue (UserInterface|CreateWidget "/Game/DapperStapper/Quiz/Widgets/WBP_QuizMenu.WBP_QuizMenu_C" 0 (.question (Utilities|Array|Get(acopy) (.quizquestion (.Value (Utilities|Map|Find (Variables|Quiz|GetQuizQuestions) LocationName))) (Variables|Quiz|GetCurrentQuestion)))))
  (Components|Animation|PlayAnimation _quizinfomesh (.mascotanimation (Utilities|Array|Get(acopy) (.quizquestion (.Value (Utilities|Map|Find (Variables|Quiz|GetQuizQuestions) LocationName))) (Variables|Quiz|GetCurrentQuestion))) (select (and (!= (.mascotanimation (Utilities|Array|Get(acopy) (.quizquestion (.Value (Utilities|Map|Find (Variables|Quiz|GetQuizQuestions) LocationName))) (Variables|Quiz|GetCurrentQuestion))) "/Game/DapperStapper/Art/Pieter_Paaltje/Animaties/SM_Pieter_Anim_Pieter_Bones_Pieter_Exit.SM_Pieter_Anim_Pieter_Bones_Pieter_Exit") (!= (.mascotanimation (Utilities|Array|Get(acopy) (.quizquestion (.Value (Utilities|Map|Find (Variables|Quiz|GetQuizQuestions) LocationName))) (Variables|Quiz|GetCurrentQuestion))) "/Game/DapperStapper/Art/Pieter_Paaltje/Animaties/SM_Pieter_Anim_Pieter_Bones_Pieter_Entry.SM_Pieter_Anim_Pieter_Bones_Pieter_Entry")) true false))
  (Rendering|SetVisibility _quizinfomesh true false)
  (bind _output_get (Variables|References|SetQuizMenuRef _returnvalue))
  (UserInterface|Viewport|AddtoViewport _output_get 0)
  (for _array_element (.answers (Utilities|Array|Get(acopy) (.quizquestion (.Value (Utilities|Map|Find (Variables|Quiz|GetQuizQuestions) LocationName))) (Variables|Quiz|GetCurrentQuestion)))
    (Default|AddButton (Variables|References|GetQuizMenuRef) (.answer _array_element) (.correct? _array_element)))
  (return))

(fn PutCollectableonScreen
  (params (CollectableMesh :type Static%20Mesh%20Object%20Reference) (InFloat :type Float%20%28single-precision%29) (LocationToCheck :type E_LocationEnum%20Enum%20%28by%20ref%29 :default "NewEnumerator3"))
  (bind _returnvalue (Utilities|GetDisplayName CollectableMesh))
  (bind _playerref (Variables|References|GetPlayerRef))
  (bind _returnvalue_2 (Utilities|String|RightChop _returnvalue 3))
  (bind _itemmesh (Variables|/Game/TopDownBP/Blueprints/TopDownCharacter.TopDownCharacter_C|GetItemMesh _playerref))
  ;[1 1 1] Creates the "CollectableAcquired" menu with the right collectable and text.
  (Widget|RemovefromParent (Variables|/Game/TopDownBP/Blueprints/TopDownCharacter.TopDownCharacter_C|GetInventoryWidgetRef (Variables|References|GetPlayerRef)))
  (Utilities|Platform|CollectGarbage)
  (Rendering|SetVisibility (Variables|/Game/TopDownBP/Blueprints/TopDownCharacter.TopDownCharacter_C|GetQuizInfoMesh (Variables|References|GetPlayerRef)) false false)
  (Components|StaticMesh|SetStaticMesh _itemmesh CollectableMesh)
  (Transformation|SetWorldScale3D _itemmesh (Math|Conversions|ToVector(Float) InFloat))
  ;;[0 0 0] Adds widget for the text below a collectable.
  (bind _returnvalue_3 (UserInterface|CreateWidget "/Game/DapperStapper/Quiz/Widgets/WBP_CollectableAcquired.WBP_CollectableAcquired_C" 0 (select (.Value (Utilities|Map|Find (Variables|/Game/DapperStapper/Save/BP_SaveGame.BP_SaveGame_C|GetCollectionMap (Variables|/Game/DapperStapper/Save/BP_SaveManager.BP_SaveManager_C|GetSaveGameRef (Variables|References|GetSaveManagerRef))) LocationToCheck)) (Utilities|Text|ToText(String) (Utilities|String|Append "Je hebt " _returnvalue_2 " al in je verzameling.")) (Utilities|Text|ToText(String) (Utilities|String|Append "Gefeliciteerd! Je hebt " _returnvalue_2 " gevonden.")))))
  (bind _output_get (Variables|References|SetCollectableAcquiredRef _returnvalue_3))
  (UserInterface|Viewport|AddtoViewport _output_get 0)
  (Variables|Collectables|SetCollectableOnScreen true)
  (return))