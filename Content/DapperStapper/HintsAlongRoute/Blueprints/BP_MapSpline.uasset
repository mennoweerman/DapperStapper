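; BP_MapSpline is an actor that gives the player a hint along the route and advances saved progress.
; On BeginPlay it caches the TopDownCharacter and BP_SaveManager.
; GiveHintToPlayer removes the inventory widget and, if hint text exists, shows WBP_HintMenu and applies the hint's static and skeletal meshes to the character's item components.
; It then increments the saved LocationIndex, disables the character's Plane collision, sets game-only input and saves.
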(event EventBeginPlay
  ;[1 1 1] Sets a reference to the character
  (bind _astop_down_character (Utilities|Casting|CastToTopDownCharacter (Game|GetPlayerCharacter 0)))
  (Variables|References|SetCharacterRef _astop_down_character)
  (bind _returnvalue (Actor|GetActorOfClass "/Game/DapperStapper/Save/BP_SaveManager.BP_SaveManager_C"))
  (Variables|References|SetSaveManagerRef _returnvalue))

(event Collision|EventActorBeginOverlap
  (params (OtherActor :type Actor%20Object%20Reference)))

(fn ConstructionScript)

(fn GiveHinttoPlayer
  (bind _hinttext (Variables|Hints|GetHintText))
  (bind _savemanagerref (Variables|References|GetSaveManagerRef))
  (bind _characterref (Variables|References|GetCharacterRef))
  (bind _hintskeletalmesh (Variables|Hints|GetHintSkeletalMesh))
  (bind _itemmesh (Variables|/Game/TopDownBP/Blueprints/TopDownCharacter.TopDownCharacter_C|GetItemMesh _characterref))
  (bind _skeletalitemmesh (Variables|/Game/TopDownBP/Blueprints/TopDownCharacter.TopDownCharacter_C|GetSkeletalItemMesh _characterref))
  ;[1 1 1] Checks if the player is close to a point where a hint can be given. Manages the widget for the hints.
  (Widget|RemovefromParent (Variables|/Game/TopDownBP/Blueprints/TopDownCharacter.TopDownCharacter_C|GetInventoryWidgetRef (Variables|References|GetCharacterRef)))
  (Utilities|Platform|CollectGarbage)
  (if (not (Utilities|Text|TextIsEmpty _hinttext))
    (bind _returnvalue (UserInterface|CreateWidget "/Game/DapperStapper/HintsAlongRoute/Widgets/WBP_HintMenu.WBP_HintMenu_C" 0 _hinttext))
    (bind _output_get (Variables|References|SetHintMenuRef _returnvalue))
    (UserInterface|Viewport|AddtoViewport _output_get 0)
    (Components|StaticMesh|SetStaticMesh _itemmesh (Variables|Hints|GetHintMesh))
    (Class|SkinnedMeshComponent|SetSkeletalMesh _skeletalitemmesh _hintskeletalmesh true)
    (Transformation|SetWorldScale3D _itemmesh (Math|Conversions|ToVector(Float) (Variables|Hints|GetHintMeshScale)))
    (if (== _hintskeletalmesh _skeletalitemmesh)
      (Components|Animation|PlayAnimation _skeletalitemmesh "/Game/DapperStapper/Art/Been/Animaties/Been_Animatie_02.Been_Animatie_02" true))
    (Math|Integer|IncrementInt (Variables|/Game/DapperStapper/Save/BP_SaveGame.BP_SaveGame_C|GetLocationIndex (Variables|/Game/DapperStapper/Save/BP_SaveManager.BP_SaveManager_C|GetSaveGameRef _savemanagerref))
      (:%20%20
        (Collision|SetCollisionEnabled (Variables|/Game/TopDownBP/Blueprints/TopDownCharacter.TopDownCharacter_C|GetPlane (Variables|References|GetCharacterRef)) "NoCollision")
        (Input|SetInputModeGameOnly (Game|GetPlayerController 0))
        (Default|SaveGame _savemanagerref)
        (return)))))