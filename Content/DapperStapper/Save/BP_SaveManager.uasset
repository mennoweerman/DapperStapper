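; BP_SaveManager owns the game's save data and shows the intro when the game level starts without it having been played.
; On BeginPlay it loads the BP_SaveGame from the named slot, or creates a new save object if none exists.
; If the current level is the game level and IntroPlayed is false, it adds a WBP_GameIntro widget.
; A SaveGame event writes the held save object back to the slot.
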(event Custom|Save%20Game
  ;[1 1 1] Event that saves the game to the save file of choice
  (SaveGame|SaveGametoSlot (Variables|SaveFileReferences|GetSaveGameRef) (Variables|SaveFileReferences|GetSaveFileName)))

(event EventBeginPlay
  ;[1 1 1] Creates or loads save on begin play
  (CallFunction|CreateorLoadSave)
  (bind _returnvalue (Game|GetCurrentLevelName true))
  ;[1 1 1] If the intro is not played and if the gamelevel is open, create the intro widget
  (if (and (Utilities|Enum|Equal(Enum) _returnvalue (Variables|IntroSettings|GetGameLevelName)) (not (Variables|/Game/DapperStapper/Save/BP_SaveGame.BP_SaveGame_C|GetIntroPlayed? (Variables|SaveFileReferences|GetSaveGameRef))))
    (bind _returnvalue_2 (UserInterface|CreateWidget "/Game/DapperStapper/GameIntro/Widgets/WBP_GameIntro.WBP_GameIntro_C" 0 (Variables|IntroSettings|GetIntroArray)))
    (UserInterface|Viewport|AddtoViewport _returnvalue_2 0)))

(fn ConstructionScript)

(fn CreateorLoadSave
  ;[1 1 1] Checks if save file exists, if not then creates a savefile. Otherwise loading the save file
  (bind _returnvalue (SaveGame|DoesSaveGameExist (Variables|SaveFileReferences|GetSaveFileName)))
  (if _returnvalue
    (bind _returnvalue_2 (SaveGame|LoadGamefromSlot (Variables|SaveFileReferences|GetSaveFileName)))
    (bind _asbp_save_game (Utilities|Casting|CastToBP_SaveGame _returnvalue_2))
    (Variables|SaveFileReferences|SetSaveGameRef _asbp_save_game)
    (else
      (bind _returnvalue_3 (SaveGame|CreateSaveGameObject "/Game/DapperStapper/Save/BP_SaveGame.BP_SaveGame_C"))
      (Variables|SaveFileReferences|SetSaveGameRef _returnvalue_3))))