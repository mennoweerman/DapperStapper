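; BP_Inventory is an actor that shows the player's saved collectables on the TopDownCharacter.
; SpawnInventory matches CollectableHolder component names to enum keys in BP_SaveManager's CollectionMap, unhides those marked collected, then triggers a size change.
; A bound event plays or reverses a timeline that scales the holder's children, showing the player's Plane while open and hiding it after closing.
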(event Custom|StartSizeChange_Event
  (params (IncreaseSize? :type Boolean))
  ;[1 1 1] Change collectable size
  (if IncreaseSize?
    (Development|SetHiddeninGame (Variables|/Game/TopDownBP/Blueprints/TopDownCharacter.TopDownCharacter_C|GetPlane (Variables|References|GetPlayerRef)) false false)
    (bind _collectablecurve (Timeline|Timeline_0 PlayFromStart)
      (:Update
        (for _array_element (Components|GetChildrenComponents (Variables|/Game/TopDownBP/Blueprints/TopDownCharacter.TopDownCharacter_C|GetCollectableHolder (Variables|References|GetPlayerRef)) false)
          (Transformation|SetRelativeScale3D _array_element (Math|Vector|MakeVector _collectablecurve _collectablecurve _collectablecurve))))
      (:Finished
        (if (not IncreaseSize?)
          (Development|SetHiddeninGame _array_element true false))))
    (else
      (Timeline|Timeline_0 ReverseFromEnd))))

(event EventBeginPlay
  ;[1 1 1] Set references
  (bind _returnvalue (Actor|GetActorOfClass "/Game/DapperStapper/Save/BP_SaveManager.BP_SaveManager_C"))
  (Utilities|IsValid _returnvalue
    (:Is%20Valid
      (Variables|References|SetSaveManagerRef _returnvalue)
      (bind _returnvalue_2 (Actor|GetActorOfClass "/Game/TopDownBP/Blueprints/TopDownCharacter.TopDownCharacter_C"))
      (Variables|References|SetPlayerRef _returnvalue_2)
      ;[1 1 1] Change collectable size
      (EventDispatchers|BindEventtoStartSizeChange (delegate Custom|StartSizeChange_Event)))
    (:Is%20Not%20Valid
      (Development|PrintString "ERROR: BP_SaveManager not found in map! Inventory button will not function." true true "(R=1.000000,G=0.000000,B=0.000000,A=1.000000)" 1e+01))))

(fn ConstructionScript)

(fn SpawnInventory
  (bind _savemanagerref (Variables|References|GetSaveManagerRef))
  (bind _savegameref (Variables|/Game/DapperStapper/Save/BP_SaveManager.BP_SaveManager_C|GetSaveGameRef _savemanagerref))
  (bind _collectionmap (Variables|/Game/DapperStapper/Save/BP_SaveGame.BP_SaveGame_C|GetCollectionMap _savegameref))
  ;[1 1 1] Check the save file for collected collectables and make them visible
  (for _array_element (Components|GetChildrenComponents (Variables|/Game/TopDownBP/Blueprints/TopDownCharacter.TopDownCharacter_C|GetCollectableHolder (Variables|References|GetPlayerRef)) true)
    (bind _keys (Utilities|Map|Keys _collectionmap))
    (bind _array_element_2 (Utilities|Array|ForEachLoopwithBreak _keys :!label _label)
      (:LoopBody
        (if (Utilities|Enum|Equal(Enum) (Utilities|String|EnumtoString _array_element_2) (Utilities|GetObjectName _array_element))
          (LocalVariables|SetLoopBroken true)
          (goto _label Break)))
      (:Completed
        (Development|SetHiddeninGame _array_element (not (and (LocalVariables|GetLoopBroken) (.Value (Utilities|Map|Find _collectionmap _array_element_2)))) false)
        (LocalVariables|SetLoopBroken false))))
  (Default|CallStartSizeChange true))