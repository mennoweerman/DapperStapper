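; BP_Inventory handles the inventory toggle event, though its spawning logic is not yet implemented.
; On BeginPlay it caches the save manager and TopDownCharacter, then binds to the HandleInventory dispatcher, or prints an error if no save manager exists.
; The event calls SpawnInventory, an empty stub with unconnected reads of the player camera location and saved CollectionMap.
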(event Custom|HandleInventory_Event
  (CallFunction|SpawnInventory))

(event EventBeginPlay
  (bind _returnvalue (Actor|GetActorOfClass "/Game/DapperStapper/Save/BP_SaveManager.BP_SaveManager_C"))
  (Utilities|IsValid _returnvalue
    (:Is%20Valid
      (Variables|Default|SetBP_SaveManagerRef _returnvalue)
      (bind _returnvalue_2 (Actor|GetActorOfClass "/Game/TopDownBP/Blueprints/TopDownCharacter.TopDownCharacter_C"))
      (Variables|Default|SetPlayerRef _returnvalue_2)
      (EventDispatchers|BindEventtoHandleInventory (delegate Custom|HandleInventory_Event)))
    (:Is%20Not%20Valid
      (Development|PrintString "ERROR: BP_SaveManager not found in map! Inventory button will not function." true true "(R=1.000000,G=0.000000,B=0.000000,A=1.000000)" 1e+01))))

(fn ConstructionScript)

(fn SpawnInventory)